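; BP_King is a destructible actor from the Tile folder that loses health when damaged.
; Any damage event calls Hurt, which decrements Health by one regardless of the damage amount.
; Hurt then switches on Health, swapping the sprite at one point left and destroying the actor at zero.
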(event EventBeginPlay
  (|CallParentFunction) ; 此节点被禁用，将不会被调用。\n从引脚连出引线来编译功能。
)

(event Collision|EventActorBeginOverlap
  (params (OtherActor :type Actor%20Object%20Reference))
  (|CallParentFunction OtherActor) ; 此节点被禁用，将不会被调用。\n从引脚连出引线来编译功能。
)

(event EventTick
  (params (DeltaSeconds :type Float%20%28single-precision%29))
  (|CallParentFunction DeltaSeconds) ; 此节点被禁用，将不会被调用。\n从引脚连出引线来编译功能。
)

(event Game|Damage|EventAnyDamage
  (params (Damage :type Float%20%28single-precision%29) (DamageType :type Damage%20Type%20Object%20Reference) (InstigatedBy :type Controller%20Object%20Reference) (DamageCauser :type Actor%20Object%20Reference))
  (CallFunction|Hurt))

(fn ConstructionScript
  (|CallParentFunction))

(fn Hurt
  (bind _result (Math|Integer|DecrementInt (Variables|Default|Gethealth))
    (:%20%20
      (bind _output_get (Variables|Default|Sethealth _result))
      (switch int _output_get
        (:0
          (Actor|DestroyActor))
        (:1
          (Rendering|Components|Sprite|SetSprite (Variables|Default|GetSprite) "/Game/Assets/Sprites/tile_scene_7.tile_scene_7"))))))