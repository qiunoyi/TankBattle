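; BF_global is a Blueprint function library of shared helpers for tile-based, four-direction movement.
; Two lookups map a direction enum to a unit vector on the XY plane, with Up as negative Y, and to a quarter-turn rotation.
; AlignTile rounds a value to tile steps, subtracting the width and dividing by the offset before scaling by width and adding the offset.
; GetGameModeBP returns the current game mode, cast to GameMode.
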(fn GetForwordbyDirection
  (params (direction :type E_direction%20Enum :default "NewEnumerator0"))
  (return (Utilities|Select :Index direction :NewEnumerator0 "0,-1.000000, 0" :NewEnumerator1 "0,1.000000, 0" :NewEnumerator2 "1.000000, 0, 0" :NewEnumerator3 "-1.000000, 0, 0" :NewEnumerator4 "0, 0, 0")))

(fn AlignTile
  (params (value :type Float%20%28single-precision%29) (tileWidth :type Float%20%28single-precision%29) (offset :type Float%20%28single-precision%29))
  (return (+ (* (Math|Float|Round (/ (- value tileWidth) offset)) tileWidth) offset)))

(fn GetRotationbyDirection
  (params (direction :type E_direction%20Enum :default "NewEnumerator0"))
  (return (Utilities|Select :Index direction :NewEnumerator0 "0, 0, 0" :NewEnumerator1 "0.000000,180.000000, 0" :NewEnumerator2 "0.000000,90.000000, 0" :NewEnumerator3 "0.000000,270.000000, 0" :NewEnumerator4 "0, 0, 0")))

(fn GetGameModeBP
  (return (.As游戏模式 (Utilities|Casting|CastToGameMode (Game|GetGameMode)))))