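; Tank movement component that drives its owning actor in four directions on a tile grid.
; MoveToDirection turns the owner to the direction, computes a velocity from Speed and flags it moving, while Tick applies the swept offset scaled by delta time.
; On each move call, the tank snaps to the tile grid on X for Up/Down or Y for Left/Right.
; Starting and stopping also send an animation status to the owner.
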(event EventBeginPlay)

(event EventTick
  (params (DeltaSeconds :type Float%20%28single-precision%29))
  (if (Variables|Default|GetisMoving)
    (Transformation|AddActorWorldOffset (Components|GetOwner) (* (Variables|Default|Getoffset) DeltaSeconds) true)))

(fn MovetoDirection
  (params (direction :type E_direction%20Enum :default "NewEnumerator0"))
  (Variables|Default|Setdirection direction)
  (CallFunction|Move)
  (Variables|Default|SetisMoving true)
  (Class|IAnimaStatus|SetAnimaStatus(Message) (Components|GetOwner) "NewEnumerator1"))

(fn Move
  (bind _returnvalue (Components|GetOwner))
  (bind _direction (Variables|Default|Getdirection))
  (bind _value (CallFunction|GetForwordbyDirection _direction))
  (Variables|Default|Setoffset (* _value (Variables|Default|Getspeed)))
  (bind _value_2 (CallFunction|GetRotationbyDirection _direction))
  (Transformation|SetActorRotation _returnvalue _value_2)
  (CallFunction|AlignTanktoTile _returnvalue _direction))

(fn StopbyDirection
  (params (direction :type E_direction%20Enum :default "NewEnumerator0"))
  (if (== direction (Variables|Default|Getdirection))
    (Variables|Default|SetisMoving false)
    (Class|IAnimaStatus|SetAnimaStatus(Message) (Components|GetOwner) "NewEnumerator0")))

(fn AlignTanktoTile
  (params (tank :type Actor%20Object%20Reference) (direction :type E_direction%20Enum :default "NewEnumerator0"))
  (bind _returnvalue (Transformation|GetActorLocation tank))
  (switch Utilities|FlowControl|Switch|SwitchonE_direction direction
    (:NewEnumerator0
      (bind _return (CallFunction|AlignTile (.x _returnvalue) 16.0 16.0 :!label _label))
      (Transformation|SetActorLocation tank (Math|Vector|MakeVector _return (.y _returnvalue) (.z _returnvalue)) false false))
    (:NewEnumerator1
      (goto _label))
    (:NewEnumerator2
      (bind _return_2 (CallFunction|AlignTile (.y _returnvalue) 16.0 16.0 :!label _label_2))
      (Transformation|SetActorLocation tank (Math|Vector|MakeVector (.x _returnvalue) _return_2 (.z _returnvalue)) false false))
    (:NewEnumerator3
      (goto _label_2))))