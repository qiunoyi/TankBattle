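; Enemy factory Blueprint for a tank game, meant to spawn a normal, quick or heavy enemy tank according to its Type.
; CreateEnemy only returns the Enemy variable, because the switch that spawns the matching class and stores it in Enemy is disconnected and never runs.
; Each spawn branch uses the same fixed transform, and BeginPlay and Tick are empty, disabled placeholders.
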(event EventBeginPlay)

(event EventTick
  (params (DeltaSeconds :type Float%20%28single-precision%29)))

(fn CreateEnemy
  (return (Variables|Default|Getenemy)))