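; Player tank Blueprint that sets idle and move animations by player index and drives player index 1 with simple AI.
; The AI runs on a one-second looping timer, storing the tank's location and sending BPMovement in a random one of four directions when it has not moved.
; Damage lowers Health, teleporting the tank to its birth location at two or one remaining and destroying it at zero.
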(event Custom|AI移动
  (bind _returnvalue (Transformation|GetActorLocation))
  (bind _bp_movement (Variables|Default|GetBP_movement))
  ;[1 1 1] 玩家AI移动
  (if (Math|Vector|Equal(Vector) (Variables|Default|GetcurLocation) _returnvalue 0.0001)
    (switch int (Math|Random|RandomInteger 4)
      (:0
        (Default|MovetoDirection _bp_movement "NewEnumerator1"))
      (:1
        (Default|MovetoDirection _bp_movement "NewEnumerator0"))
      (:2
        (Default|MovetoDirection _bp_movement "NewEnumerator2"))
      (:3
        (Default|MovetoDirection _bp_movement "NewEnumerator3")))
    (else
      (Variables|Default|SetcurLocation _returnvalue))))

(event EventBeginPlay
  ;[1 1 1] 玩家AI移动
  (|CallParentFunction)
  (if (== (Variables|config|GetplayerIndex) 1)
    (CallFunction|AI移动)
    (Utilities|Time|SetTimerbyEvent (delegate Custom|AI移动) 1.0 true)))

(event Collision|EventActorBeginOverlap
  (params (OtherActor :type Actor%20Object%20Reference))
  (|CallParentFunction OtherActor) ; 此节点被禁用，将不会被调用。\n从引脚连出引线来编译功能。
)

(event EventTick
  (params (DeltaSeconds :type Float%20%28single-precision%29))
  (|CallParentFunction DeltaSeconds) ; 此节点被禁用，将不会被调用。\n从引脚连出引线来编译功能。
)

(event EventInitAnima
  (switch int (Variables|config|GetplayerIndex)
    (:0
      (Variables|Default|SetidleAnima "/Game/Assets/Animations/Player_0_idle.Player_0_idle")
      (Variables|Default|SetmovingAnima "/Game/Assets/Animations/Player_0_Move.Player_0_move"))
    (:1
      (Variables|Default|SetidleAnima "/Game/Assets/Animations/Player_1_idle.Player_1_idle")
      (Variables|Default|SetmovingAnima "/Game/Assets/Animations/Player_1_move.Player_1_move"))))

(event Game|Damage|EventAnyDamage
  (params (Damage :type Float%20%28single-precision%29) (DamageType :type Damage%20Type%20Object%20Reference) (InstigatedBy :type Controller%20Object%20Reference) (DamageCauser :type Actor%20Object%20Reference))
  (bind _output_get (Variables|Default|Sethealth (- (Variables|Default|Gethealth) (Math|Float|Truncate Damage))))
  (switch int _output_get
    (:0
      (Actor|DestroyActor))
    (:1
      (Transformation|SetActorLocation (Variables|Default|GetbirthLocation) false false :!label _label))
    (:2
      (goto _label))))

(fn ConstructionScript
  (|CallParentFunction))