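; BP_tank is a 2D tank that moves in four directions and fires bullets.
; Directional input actions drive its BPMovement component, and SetAnimaStatus swaps the Paper2D flipbook between idle and moving, with InitAnima left as an empty hook.
; Shoot spawns a BP_bullet along the movement direction, from NumPad 0 or an optional looping auto-fire timer.
; Both triggers fire only when the previous bullet is no longer valid, limiting the tank to one live shot.
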(event Custom|initAnima)

(event Custom|自动射击
  ;[1 1 1] 自动射击
  (if (not (Utilities|IsValid (Variables|Default|Getbullets)))
    (CallFunction|Shoot)))

(event EventBeginPlay
  (CallFunction|InitAnima)
  (CallFunction|SetAnimaStatus "NewEnumerator0")
  ;[1 1 1] 自动射击
  (if (Variables|Default|GetautoShoot)
    (CallFunction|自动射击)
    (Utilities|Time|SetTimerbyEvent (delegate Custom|自动射击) 0.5 true)))

(event Collision|EventActorBeginOverlap
  (params (OtherActor :type Actor%20Object%20Reference)))

(event EventTick
  (params (DeltaSeconds :type Float%20%28single-precision%29)))

(event EventSetAnimaStatus
  (params (NewParam :type E_animaStatus%20Enum :default "NewEnumerator0"))
  ;[1 1 1] 设置动画状态
  (bind _output_get (Variables|Default|Setstatus NewParam))
  (Sprite|SetFlipbook (Variables|Default|Gettank) (Utilities|Select :Index _output_get :NewEnumerator0 (Variables|Default|GetidleAnima) :NewEnumerator1 (Variables|Default|GetmovingAnima))))

(event Input|ActionEvents|InputActionUp
  (params (Key :type Key%20Structure))
  (bind _bp_movement (Variables|Default|GetBP_movement))
  ;[1 1 1] 移动
  (:Pressed
    (Default|MovetoDirection _bp_movement "NewEnumerator0"))
  (:Released
    (Default|StopbyDirection _bp_movement "NewEnumerator0")))

(event Input|ActionEvents|InputActionLeft
  (params (Key :type Key%20Structure))
  (bind _bp_movement (Variables|Default|GetBP_movement))
  ;[1 1 1] 移动
  (:Pressed
    (Default|MovetoDirection _bp_movement "NewEnumerator3"))
  (:Released
    (Default|StopbyDirection _bp_movement "NewEnumerator3")))

(event Input|ActionEvents|InputActionRight
  (params (Key :type Key%20Structure))
  (bind _bp_movement (Variables|Default|GetBP_movement))
  ;[1 1 1] 移动
  (:Pressed
    (Default|MovetoDirection _bp_movement "NewEnumerator2"))
  (:Released
    (Default|StopbyDirection _bp_movement "NewEnumerator2")))

(event Input|ActionEvents|InputActionDown
  (params (Key :type Key%20Structure))
  (bind _bp_movement (Variables|Default|GetBP_movement))
  ;[1 1 1] 移动
  (:Pressed
    (Default|MovetoDirection _bp_movement "NewEnumerator1"))
  (:Released
    (Default|StopbyDirection _bp_movement "NewEnumerator1")))

(event Input|KeyboardEvents|NumPadZero
  (params (Key :type Key%20Structure))
  ;[1 1 1] 手动射击
  (:Pressed
    (if (not (Utilities|IsValid (Variables|Default|Getbullets)))
      (CallFunction|Shoot))))

(fn ConstructionScript)

(fn Shoot
  (bind _self self)
  (bind _returnvalue (Game|SpawnActorfromClass "/Game/Blueprint/tank/BP_bullet.BP_bullet_C" (Transformation|GetActorTransform) "Undefined" _self (Variables|/Game/Blueprint/tank/BP_movement.BP_movement_C|Getdirection (Variables|Default|GetBP_movement)) 2.5e+02 _self))
  (Variables|Default|Setbullets _returnvalue))

(fn GetAnimaStatus
  (return (Variables|Default|Getstatus)))