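; Heavy enemy tank Blueprint, a child class that sets its own idle and moving flipbooks and movement speed in the construction script.
; Any damage is truncated to an integer and subtracted from Health, then SetHurtAnima switches on the exact remaining value.
; Low health swaps in yellow, then red hurt flipbooks, and exactly zero destroys the actor, so negative Health matches no case.
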(event EventBeginPlay
  (|CallParentFunction) ; 此节点被禁用，将不会被调用。\n从引脚连出引线来编译功能。
)

(event Collision|EventActorBeginOverlap
  (params (OtherActor :type Actor%20Object%20Reference))
  (|CallParentFunction OtherActor) ; 此节点被禁用，将不会被调用。\n从引脚连出引线来编译功能。
)

(event EventTick
  (params (DeltaSeconds :type Float%20%28single-precision%29))
  (|CallParentFunction DeltaSeconds) ; 此节点被禁用，将不会被调用。\n从引脚连出引线来编译功能。
)

(event EventInitAnima)

(event Game|Damage|EventAnyDamage
  (params (Damage :type Float%20%28single-precision%29) (DamageType :type Damage%20Type%20Object%20Reference) (InstigatedBy :type Controller%20Object%20Reference) (DamageCauser :type Actor%20Object%20Reference))
  (Variables|Default|Sethealth (- (Variables|Default|Gethealth) (Math|Float|Truncate Damage)))
  (CallFunction|SetHurtAnima))

(fn ConstructionScript
  (|CallParentFunction)
  (Variables|Default|SetidleAnima "/Game/Assets/Animations/Enemy_2_idle.Enemy_2_idle")
  (Variables|Default|SetmovingAnima "/Game/Assets/Animations/Enemy_2_moving.Enemy_2_moving")
  (Variables|/Game/Blueprint/tank/BP_movement.BP_movement_C|Setspeed (Variables|Default|GetBP_movement) 44.0))

(fn SetHurtAnima
  (switch int (Variables|Default|Gethealth)
    (:0
      (Actor|DestroyActor))
    (:1
      (bind _output_get (Variables|Default|SetidleAnima "/Game/Assets/Animations/redHurt2_idle.redHurt2_idle"))
      (Variables|Default|SetmovingAnima "/Game/Assets/Animations/redHurt2_moving.redHurt2_moving")
      (Sprite|SetFlipbook (Variables|Default|Gettank) _output_get))
    (:2
      (bind _output_get_2 (Variables|Default|SetidleAnima "/Game/Assets/Animations/YellowHurt2_idle.YellowHurt2_idle"))
      (Variables|Default|SetmovingAnima "/Game/Assets/Animations/YellowHurt2_moving.YellowHurt2_moving")
      (Sprite|SetFlipbook (Variables|Default|Gettank) _output_get_2))))