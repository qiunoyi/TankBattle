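; Tank bullet actor that flies in a set direction and deals damage on contact.
; Construction derives a velocity offset from Direction and Speed and rotates the owner to that direction; Tick moves the bullet with sweep.
; BeginPlay makes the bullet and its owner's boxes ignore each other while moving.
; Hits always damage and destroy the bullet; overlaps skip damage when the other actor's tags match the owner's.
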(event OnComponentBeginOverlap(Box)
  (params (OverlappedComponent :type Primitive%20Component%20Object%20Reference) (OtherActor :type Actor%20Object%20Reference) (OtherComp :type Primitive%20Component%20Object%20Reference) (OtherBodyIndex :type Integer) (bFromSweep :type Boolean) (SweepResult :type Hit%20Result%20Structure%20%28by%20ref%29))
  (if (Utilities|Array|Identical (Variables|/Script/Engine.Actor|GetTags (Components|GetOwner)) (Variables|/Script/Engine.Actor|GetTags OtherActor))
    (Actor|DestroyActor)
    (else
      (Game|Damage|ApplyDamage OtherActor 1.0 0 0)
      (Actor|DestroyActor))))

(event OnComponentHit(Box)
  (params (HitComponent :type Primitive%20Component%20Object%20Reference) (OtherActor :type Actor%20Object%20Reference) (OtherComp :type Primitive%20Component%20Object%20Reference) (NormalImpulse :type Vector :default "0, 0, 0") (Hit :type Hit%20Result%20Structure%20%28by%20ref%29))
  (Game|Damage|ApplyDamage OtherActor 1.0 0 0)
  (Actor|DestroyActor))

(event EventBeginPlay
  (bind _returnvalue (Components|GetOwner))
  (Collision|IgnoreActorwhenMoving (Variables|Default|GetBox) _returnvalue true)
  (Collision|IgnoreActorwhenMoving (Actor|GetComponentsByClass _returnvalue "/Script/Engine.BoxComponent") self true))

(event Collision|EventActorBeginOverlap
  (params (OtherActor :type Actor%20Object%20Reference)))

(event EventTick
  (params (DeltaSeconds :type Float%20%28single-precision%29))
  (Transformation|AddActorWorldOffset (* (Variables|Default|Getoffset) DeltaSeconds) true))

(fn ConstructionScript
  (bind _direction (Variables|Default|Getdirection))
  (bind _value (CallFunction|GetForwordbyDirection _direction))
  (Variables|Default|Setoffset (* _value (Variables|Default|Getspeed)))
  (bind _value_2 (CallFunction|GetRotationbyDirection _direction))
  (Transformation|SetActorRotation (Components|GetOwner) _value_2))