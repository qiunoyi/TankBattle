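; BP_ememy_quick is a fast enemy tank variant, built as a child Blueprint that configures inherited behavior.
; Its construction script runs the parent's, then assigns the Enemy_0 idle and moving animations and sets the BPMovement speed.
; Any damage destroys the actor outright, with no health check.
; The InitAnima event is present but empty, and BeginPlay, overlap and Tick are disabled placeholder nodes.
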(event EventBeginPlay
  (|CallParentFunction) ; 此节点被禁用，将不会被调用。\n从引脚连出引线来编译功能。
)

(event Collision|EventActorBeginOverlap
  (params (OtherActor :type Actor%20Object%20Reference))
  (|CallParentFunction OtherActor) ; 此节点被禁用，将不会被调用。\n从引脚连出引线来编译功能。
)

(event EventTick
  (params (DeltaSeconds :type Float%20%28single-precision%29))
  (|CallParentFunction DeltaSeconds) ; 此节点被禁用，将不会被调用。\n从引脚连出引线来编译功能。
)

(event EventInitAnima)

(event Game|Damage|EventAnyDamage
  (params (Damage :type Float%20%28single-precision%29) (DamageType :type Damage%20Type%20Object%20Reference) (InstigatedBy :type Controller%20Object%20Reference) (DamageCauser :type Actor%20Object%20Reference))
  (Actor|DestroyActor))

(fn ConstructionScript
  (|CallParentFunction)
  (Variables|Default|SetidleAnima "/Game/Assets/Animations/Enemy_0_idle.Enemy_0_idle")
  (Variables|Default|SetmovingAnima "/Game/Assets/Animations/Enemy_0_moving.Enemy_0_moving")
  (Variables|/Game/Blueprint/tank/BP_movement.BP_movement_C|Setspeed (Variables|Default|GetBP_movement) 176.0))