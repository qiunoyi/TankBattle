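; Normal enemy tank that uses Paper2D flipbooks for its idle and moving animations.
; The construction script runs the parent's, then assigns the Enemy_1 flipbooks.
; AnyDamage subtracts truncated damage from Health and calls SetHurtAnima, which switches to red hurt flipbooks at 1 and destroys the actor at exactly 0.
; InitAnima is empty, and the BeginPlay, overlap and Tick events are disabled.
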(event EventBeginPlay
  (|CallParentFunction) ; 此节点被禁用，将不会被调用。\n从引脚连出引线来编译功能。
)

(event Collision|EventActorBeginOverlap
  (params (OtherActor :type Actor%20Object%20Reference))
  (|CallParentFunction OtherActor) ; 此节点被禁用，将不会被调用。\n从引脚连出引线来编译功能。
)

(event EventTick
  (params (DeltaSeconds :type Float%20%28single-precision%29))
  (|CallParentFunction DeltaSeconds) ; 此节点被禁用，将不会被调用。\n从引脚连出引线来编译功能。
)

(event EventInitAnima)

(event Game|Damage|EventAnyDamage
  (params (Damage :type Float%20%28single-precision%29) (DamageType :type Damage%20Type%20Object%20Reference) (InstigatedBy :type Controller%20Object%20Reference) (DamageCauser :type Actor%20Object%20Reference))
  (Variables|Default|Sethealth (- (Variables|Default|Gethealth) (Math|Float|Truncate Damage)))
  (CallFunction|SetHurtAnima))

(fn ConstructionScript
  (|CallParentFunction)
  (Variables|Default|SetidleAnima "/Game/Assets/Animations/Enemy_1_idle.Enemy_1_idle")
  (Variables|Default|SetmovingAnima "/Game/Assets/Animations/Enemy_1_moving.Enemy_1_moving"))

(fn SetHurtAnima
  (switch int (Variables|Default|Gethealth)
    (:0
      (Actor|DestroyActor))
    (:1
      (bind _output_get (Variables|Default|SetidleAnima "/Game/Assets/Animations/redHurt1_idle.redHurt1_idle"))
      (Variables|Default|SetmovingAnima "/Game/Assets/Animations/redHurt1_moving.redHurt1_moving")
      (Sprite|SetFlipbook (Variables|Default|Gettank) _output_get))))